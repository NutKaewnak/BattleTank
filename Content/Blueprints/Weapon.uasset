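; Weapon Blueprint that fires projectiles automatically while its trigger is held.
; PullTrigger passes a DoOnce gate, fires immediately, then starts a looping timer on Fire with an interval derived from RoundPerSecond.
; Fire spawns the Projectile class at the ProjectileSpawnPoint transform.
; ReleaseTrigger clears the timer and resets the gate, so nothing here limits the fire rate across repeated pulls.
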(event Custom|Fire
  ;[1 1 1] FireProjectile
  (Game|SpawnActorfromClass (Variables|Default|GetProjectile) (Transformation|GetWorldTransform (Variables|Default|GetProjectileSpawnPoint)) "Undefined" 0 0))

(event Custom|PullTrigger
  ;[1 1 1] Gun triggger
  (Utilities|FlowControl|DoOnce true
    (:Completed
      (CallFunction|Fire)
      (Utilities|Time|SetTimerbyFunctionName 0 "Fire" (/ 1.0 (Variables|Default|GetRoundPerSecond)) true))))

(event Custom|ReleaseTrigger
  ;[1 1 1] Gun triggger
  (Utilities|Time|ClearTimerbyFunctionName 0 "Fire")
  (Utilities|FlowControl|DoOnce true) ; enters at Reset
)

(event EventBeginPlay)

(event Collision|EventActorBeginOverlap
  (params (OtherActor :type Actor%20Object%20Reference)))

(event EventTick
  (params (DeltaSeconds :type Float%20%28single-precision%29)))

(fn ConstructionScript)