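; Enemy character that carries a spawned weapon and can be killed by damage.
; On BeginPlay it spawns the weapon at the GunTemp component, sets its projectile to EnemyProjectile and attaches it to GunTemp.
; AffectHealth passes the delta to CalculateHealth, then destroys both the weapon and the character if IsDead is set.
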(event EventBeginPlay
  (bind _guntemp (Variables|Default|GetGunTemp))
  ;[1 1 1] Spawn Weapon
  (bind _returnvalue (Game|SpawnActorfromClass "/Game/Blueprints/Weapon.Weapon_C" (Transformation|GetWorldTransform _guntemp) "Undefined" 0 0))
  (bind _output_get (Variables|Default|SetWeapon _returnvalue))
  (Variables|/Game/Blueprints/Weapon.Weapon_C|SetProjectile _output_get "/Game/Blueprints/EnemyProjectile.EnemyProjectile_C")
  (Transformation|AttachComponentToComponent _output_get _guntemp "None" "SnapToTarget" "KeepRelative" "KeepWorld" true))

(event Collision|EventActorBeginOverlap
  (params (OtherActor :type Actor%20Object%20Reference)))

(event EventTick
  (params (DeltaSeconds :type Float%20%28single-precision%29)))

(event EventAffectHealth
  (params (Delta :type Float%20%28single-precision%29))
  ;[1 1 1] Damaged
  (Class|BaseCharacter|CalculateHealth Delta)
  (if (Variables|Default|GetisDead)
    (Actor|DestroyActor (Variables|Default|GetWeapon))))

(fn ConstructionScript)