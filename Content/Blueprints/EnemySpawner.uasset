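; Enemy spawner actor that places EnemyCharacter AI pawns at random points inside its SpawnVolume bounds.
; Its SpawnEnemy event spawns one only while the live enemy count is under a fixed cap and MainGame's EnemyLeft counter is not negative, decrementing that counter first.
; Nothing in this Blueprint calls SpawnEnemy, as BeginPlay and Tick are unused.
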(event Custom|SpawnEnemy
  (bind _spawnvolume (Variables|Default|GetSpawnVolume))
  (bind _outactors (Actor|GetAllActorsOfClass "/Game/Blueprints/EnemyCharacter.EnemyCharacter_C"))
  (if (<= (Utilities|Array|Length _outactors) 6)
    (bind _asmain_game (Utilities|Casting|CastToMainGame (Game|GetGameMode)))
    (if (>= (Variables|/Game/MainGame.MainGame_C|GetEnemyLeft _asmain_game) 0)
      (Variables|/Game/MainGame.MainGame_C|SetEnemyLeft _asmain_game (- (Variables|/Game/MainGame.MainGame_C|GetEnemyLeft _asmain_game) 1))
      (AI|SpawnAIFromClass "/Game/Blueprints/EnemyCharacter.EnemyCharacter_C" 0 (Math|Random|RandomPointinBoundingBox (Transformation|GetWorldLocation _spawnvolume) (Components|Box|GetScaledBoxExtent _spawnvolume)) "0, 0, 0" false))))

(event EventBeginPlay)

(event Collision|EventActorBeginOverlap
  (params (OtherActor :type Actor%20Object%20Reference)))

(event EventTick
  (params (DeltaSeconds :type Float%20%28single-precision%29)))

(fn ConstructionScript)